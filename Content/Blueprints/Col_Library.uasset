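; Col_Library is a display actor that shows a material on a cube, labelled with the material's name and its physical material.
; The Construction Script applies the Material variable to the cube, then reads it back to fill two text renders, so the labels refresh whenever construction reruns.
; The event graph holds only disabled placeholder events, with no gameplay logic.
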(fn `UserConstructionScript`
  (bind _returnvalue (`PrimitiveComponent.GetMaterial` (`self.Cube`) 0))
  (`PrimitiveComponent.SetMaterial` (`self.Cube`) 0 (`self.Material`))
  (`TextRenderComponent.K2_SetText` (`self.TextRender`) (`KismetTextLibrary.Conv_StringToText` (`KismetSystemLibrary.GetDisplayName` _returnvalue)))
  (`TextRenderComponent.K2_SetText` (`self.TextRender1`) (`KismetTextLibrary.Conv_ObjectToText` (`MaterialInterface.GetPhysicalMaterial` _returnvalue))))