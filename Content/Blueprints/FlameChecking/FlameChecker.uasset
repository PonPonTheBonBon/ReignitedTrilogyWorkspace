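; FlameChecker is an actor that detects what the player's Spyro-style fire attack hits.
; On BeginPlay it snaps its root to the head socket of the BP_CPS1999_Playable mesh, so its Box follows the head.
; Shortly after FireAttack is pressed, it confirms the fire montage is playing, then sends the FlamedMessage interface call to every actor overlapping the Box except the player.
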(event `InputAction|FireAttack` :consume false :overrideparent false
  (params (Key :type "Key Structure"))
  (:`Pressed`
    (`KismetSystemLibrary.Delay` 0.2)
    (`KismetSystemLibrary.PrintString` "LeftClick")
    (bind _returnvalue (`Character.GetCurrentMontage` (cast `/CPS1999_Spyro/Blueprints/BP_CPS1999_Playable` (`GameplayStatics.GetPlayerCharacter` 0) :!pure true)))
    (if (== _returnvalue "/CPS1999_Spyro/Animations/Montages/AM_CPS1999_Fire.AM_CPS1999_Fire")
      (for _array_element (`PrimitiveComponent.GetOverlappingActors` (`self.Box`) null)
        (if (!= _array_element (`GameplayStatics.GetPlayerCharacter` 0))
          ;[1 1 1] Use blueprint interface on the blueprints that will react to spyro's fire and add the Fire Attack event
          (message `/Game/Blueprints/FlameChecking/BPI_LevelFunctions.Flamed` _array_element))))))

(event `self.ReceiveBeginPlay`
  (bind _asbp_cps1999_playable (cast `/CPS1999_Spyro/Blueprints/BP_CPS1999_Playable` (`GameplayStatics.GetPlayerCharacter` 0)))
  (`SceneComponent.K2_AttachToComponent` (`self.DefaultSceneRoot`) (`Character.Mesh` _asbp_cps1999_playable) "head" "SnapToTarget" "KeepRelative" "KeepWorld" true))

(fn `UserConstructionScript`)