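; BP_HubExtend is a mod-loader hub piece that grows its walkable area to fit a list of levels and loads them into it.
; On BeginPlay, the original piece chains copies of itself end to end at ExtensionArrow, scaling their count at one per four levels.
; It then gathers LevelLoadArea-tagged arrows from all pieces and loads each level instance at one.
; Spawned copies carry ExtraAddedPart, so they skip both steps.
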(event `CreateExtraWalkableArea`
  (bind _returnvalue (/ (`KismetArrayLibrary.Array_LastIndex` (`self.Levels`)) 4))
  (if (not (`self.ExtraAddedPart?`))
    (if (> _returnvalue 1)
      (for _ (range (+ _returnvalue 1))
        (bind _returnvalue_2 (`|SpawnActorFromClass` "BP_HubExtend_C" (`KismetMathLibrary.MakeTransform` (`SceneComponent.K2_GetComponentLocation` (`self.ExtensionArrow`))) "Undefined" "OverrideRootScale" null true null))
        (set `self.ExtensionArrow` (`/Game/ModLoader/BP_HubExtend.ExtensionArrow` _returnvalue_2))))))

(event `self.ReceiveBeginPlay`
  (`self.CreateExtraWalkableArea`)
  (`self.LoadLevels`))

(event `LoadLevels`
  (if (not (`self.ExtraAddedPart?`))
    (bind _outactors (`GameplayStatics.GetAllActorsOfClass` "BP_HubExtend_C"))
    (for _array_element _outactors
      (`KismetArrayLibrary.Array_Append` (`self.ArrowArray`) (`self.GetComponentsByTag` _array_element "/Script/Engine.ArrowComponent" "LevelLoadArea")))
    (for (_array_element_2 _array_index) (`self.Levels`)
      (bind (_returnvalue_location _returnvalue_rotation) (`KismetMathLibrary.BreakTransform` (`SceneComponent.K2_GetComponentToWorld` (`|GetArrayItem` (`self.ArrowArray`) _array_index))))
      (`LevelStreamingKismet.LoadLevelInstance` (`KismetStringLibrary.Conv_NameToString` _array_element_2) _returnvalue_location _returnvalue_rotation))))

(fn `UserConstructionScript`)