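; Fake drop shadow actor that keeps a plane on the ground beneath the player character, in place of a real shadow.
; Each Tick it runs a short complex line trace straight down from the player's capsule against WorldStatic objects.
; On a hit it shows the plane just above the impact point; otherwise it hides it.
; The trace's debug drawing is left on.
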(event `self.ReceiveTick`
  (params (DeltaSeconds :type "Float (single-precision)"))
  (bind _plane (`self.Plane`))
  (bind _returnvalue (`SceneComponent.K2_GetComponentLocation` (`Character.CapsuleComponent` (`GameplayStatics.GetPlayerCharacter` 0))))
  (bind (_outhit _returnvalue_2) (`KismetSystemLibrary.LineTraceSingleForObjects` :`Start` _returnvalue :`End` (+ _returnvalue (0.0 0.0 -150.0)) :`ObjectTypes` (`|MakeArray` "ObjectTypeQuery1" :!type "EObjectTypeQuery Enum") :`bTraceComplex` true :`DrawDebugType` "ForDuration"))
  (if _returnvalue_2
    (`SceneComponent.SetHiddenInGame` _plane false false)
    (`SceneComponent.K2_SetWorldLocation` _plane (+ (`.ImpactPoint` (`GameplayStatics.BreakHitResult` _outhit)) (0.0 0.0 1.0)) false false)
    (else
      (`SceneComponent.SetHiddenInGame` (`self.Plane`) true false))))

(fn `UserConstructionScript`)