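; BP_SlideStop is a trigger volume that ends the player's slide, undoing the slide state held by BP_SlideStart.
; The construction script sizes the box from TriggerSize and links to the first BP_SlideStart in the level.
; On player overlap it clears the slide zone flag and speed timer, resets the anim class and walk speed, removes slide-related gameplay effects, applies side rolling, and sets StopGlide on SlideStart's BP_StopGlide child actor.
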(event `self.Box.OnComponentBeginOverlap`
  (params (OverlappedComponent :type "PrimitiveComponent Object Reference") (OtherActor :type "Actor Object Reference") (OtherComp :type "PrimitiveComponent Object Reference") (OtherBodyIndex :type Integer) (bFromSweep :type Boolean) (SweepResult :type "HitResult Structure (by ref)"))
  (bind _returnvalue (`GameplayStatics.GetPlayerCharacter` 0))
  (bind _slidestart (`self.SlideStart`))
  (bind _returnvalue_2 (`AbilitySystemBlueprintLibrary.GetAbilitySystemComponent` _returnvalue))
  (if (== OtherComp (`GameplayStatics.GetPlayerCharacter` 0))
    (set `/Game/Slide/BP_SlideStart.SlideZone` false (`self.SlideStart`))
    (`SkeletalMeshComponent.SetAnimInstanceClass` (`Character.Mesh` _returnvalue) "/CPS1999_Spyro/Blueprints/ABP_CPS1999.ABP_CPS1999_C")
    (`AbilitySystemComponent.RemoveActiveGameplayEffectBySourceEffect` _returnvalue_2 "/CharacterCommon/AbilitySystem/GameplayEffects/Spyro/GE_Spyro2IceSkating.GE_Spyro2IceSkating_C" null -1)
    (`AbilitySystemComponent.BP_ApplyGameplayEffectToSelf` :`self` _returnvalue_2 :`GameplayEffectClass` "/CharacterCommon/AbilitySystem/GameplayEffects/Spyro/GE_SpyroSideRolling.GE_SpyroSideRolling_C")
    (`AbilitySystemComponent.RemoveActiveGameplayEffectBySourceEffect` _returnvalue_2 "/CharacterCommon/AbilitySystem/GameplayEffects/Spyro/GE_SpyroSlideDown.GE_SpyroSlideDown_C" null -1)
    (`AbilitySystemComponent.RemoveActiveGameplayEffectBySourceEffect` _returnvalue_2 "/CharacterCommon/AbilitySystem/GameplayEffects/Spyro/GE_SpyroDisableGliding.GE_SpyroDisableGliding_C" null -1)
    (`KismetSystemLibrary.K2_ClearAndInvalidateTimerHandle` (`/Game/Slide/BP_SlideStart.SpeedTimer` _slidestart))
    (set `CharacterMovementComponent.MaxWalkSpeed` 268.5 (`Character.CharacterMovement` (`GameplayStatics.GetPlayerCharacter` 0)))
    (bind _asbp_stop_glide (cast `/GameplayCommon/LevelMechanics/HarmfulTerrain/BP_StopGlide` (`ChildActorComponent.ChildActor` (`/Game/Slide/BP_SlideStart.GlideActor` _slidestart))))
    (set `/GameplayCommon/LevelMechanics/HarmfulTerrain/BP_StopGlide.StopGlide` true _asbp_stop_glide)))

(fn `UserConstructionScript`
  (`BoxComponent.SetBoxExtent` (`self.Box`) (`self.TriggerSize`) true)
  (bind _outactors (`GameplayStatics.GetAllActorsOfClass` "/Game/Slide/BP_SlideStart.BP_SlideStart_C"))
  (set `self.SlideStart` (`|GetArrayItem` _outactors)))