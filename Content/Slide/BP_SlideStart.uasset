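; BP_SlideStart is a resizable trigger volume that puts the Spyro player character into a slide.
; On first overlap it flags BP_StopGlide, swaps the animation instance, applies ice-skating and glide-disable gameplay effects, and removes rolling, flying and gliding effects.
; A looping timer then keeps reapplying the walk speed cap.
; While sliding, Tick pushes the player forward whenever speed is sufficiently below that cap.
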(event `self.ReceiveTick`
  (params (DeltaSeconds :type "Float (single-precision)"))
  (bind _returnvalue (`GameplayStatics.GetPlayerCharacter` 0))
  (bind _charactermovement (`Character.CharacterMovement` _returnvalue))
  (if (`self.SlideZone`)
    (if (<= (`KismetMathLibrary.VSize` (`self.GetVelocity` (`GameplayStatics.GetPlayerCharacter` 0))) (- (`self.MaxSpeed`) 250.0))
      (set `MovementComponent.Velocity` (+ (`MovementComponent.Velocity` _charactermovement) (* (`self.GetActorForwardVector` _returnvalue) (`self.PushSpeed`))) _charactermovement))))

(event `SetSpeed`
  (set `CharacterMovementComponent.MaxWalkSpeed` (`self.MaxSpeed`) (`Character.CharacterMovement` (`GameplayStatics.GetPlayerCharacter` 0))))

(event `self.Box.OnComponentBeginOverlap`
  (params (OverlappedComponent :type "PrimitiveComponent Object Reference") (OtherActor :type "Actor Object Reference") (OtherComp :type "PrimitiveComponent Object Reference") (OtherBodyIndex :type Integer) (bFromSweep :type Boolean) (SweepResult :type "HitResult Structure (by ref)"))
  (bind _returnvalue (`GameplayStatics.GetPlayerCharacter` 0))
  (bind _returnvalue_2 (`AbilitySystemBlueprintLibrary.GetAbilitySystemComponent` _returnvalue))
  (if (`self.SlideZone`)
    _
    (elif (== OtherActor _returnvalue)
      (bind _asbp_stop_glide (cast `/GameplayCommon/LevelMechanics/HarmfulTerrain/BP_StopGlide` (`ChildActorComponent.ChildActor` (`self.GlideActor`))))
      (set `/GameplayCommon/LevelMechanics/HarmfulTerrain/BP_StopGlide.StopGlide` true _asbp_stop_glide)
      (set `self.SlideZone` true)
      (`SkeletalMeshComponent.SetAnimInstanceClass` (`Character.Mesh` _returnvalue) null)
      (`AbilitySystemComponent.BP_ApplyGameplayEffectToSelf` :`self` _returnvalue_2 :`GameplayEffectClass` "/CharacterCommon/AbilitySystem/GameplayEffects/Spyro/GE_Spyro2IceSkating.GE_Spyro2IceSkating_C" :`Level` 1.0)
      (`AbilitySystemComponent.RemoveActiveGameplayEffectBySourceEffect` _returnvalue_2 "/CharacterCommon/AbilitySystem/GameplayEffects/Spyro/GE_SpyroSideRolling.GE_SpyroSideRolling_C" null -1)
      (`AbilitySystemComponent.RemoveActiveGameplayEffectBySourceEffect` _returnvalue_2 "/CharacterCommon/AbilitySystem/GameplayEffects/Spyro/GE_SpyroFlying.GE_SpyroFlying_C" null -1)
      (`AbilitySystemComponent.RemoveActiveGameplayEffectBySourceEffect` _returnvalue_2 "/CharacterCommon/AbilitySystem/GameplayEffects/Spyro/GE_SpyroGliding.GE_SpyroGliding_C" null -1)
      (`AbilitySystemComponent.BP_ApplyGameplayEffectToSelf` :`self` _returnvalue_2 :`GameplayEffectClass` "/CharacterCommon/AbilitySystem/GameplayEffects/Spyro/GE_SpyroDisableGliding.GE_SpyroDisableGliding_C" :`Level` 1.0)
      (bind _returnvalue_3 (`KismetSystemLibrary.K2_SetTimer` null "SetSpeed" 0.1 true))
      (set `self.SpeedTimer` _returnvalue_3))))

(fn `UserConstructionScript`
  (`BoxComponent.SetBoxExtent` (`self.Box`) (`self.TriggerSize`) true))